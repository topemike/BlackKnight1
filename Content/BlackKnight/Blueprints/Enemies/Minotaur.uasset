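; Minotaur enemy Blueprint whose death ends the game and rolls the credits, acting as a final boss.
; When the health component reports zero or less, it clears all widgets and has that component destroy the actor and its sprite, spawning a death explosion.
; It then shows the Credits widget on the player screen and switches the first player to UI-only input with a visible cursor.
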(event `self.HealthComponent.HealthChanged`
  (params (`New Value` :type Integer) (Change :type "/Game/Pixel2D/Blueprints/Enums/E_StatChange Enum" :default "NewEnumerator0") (Instigator :type "Actor Object Reference"))
  (bind _returnvalue (`GameplayStatics.GetPlayerController` 0))
  (if (<= `New Value` 0)
    (`WidgetLayoutLibrary.RemoveAllWidgets`)
    (`/Game/Pixel2D/Blueprints/Components/BP_HealthComponent.DestroyActorOnDeath` (`self.HealthComponent`) self (`self.PixelComponent`) 0.0 (`|MakeArray` "/Game/Pixel2D/Blueprints/Objects/BP_DeathExplode.BP_DeathExplode_C" :!type "Actor Class Reference") null null)
    (bind _returnvalue_2 (`|CreateWidget` "/Game/BlackKnight/Blueprints/credits.credits_C" _returnvalue))
    (`UserWidget.AddToPlayerScreen` _returnvalue_2 0)
    (`WidgetBlueprintLibrary.SetInputMode_UIOnlyEx` _returnvalue null)
    (set `PlayerController.bShowMouseCursor` true _returnvalue)))

(fn `UserConstructionScript`
  (`parent.UserConstructionScript`))