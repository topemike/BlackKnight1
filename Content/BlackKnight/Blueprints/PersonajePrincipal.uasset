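; Main player character Blueprint for a 2D side-scroller, handling movement, jumping and a melee attack through flipbook swaps.
; Input drives a movement component with custom Move and Jump calls, flipping control yaw to face left or right.
; Q starts the attack flipbook and flag; separate events run the AttackComponent trace and clear the flag.
; BeginPlay sets the camera view target and game-only input; pause-menu logic is unconnected.
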(event `MeleeAnimationfinished`
  (set `self.meleeattack` false))

(event `Key|Q`
  (params (Key :type "Key Structure"))
  (:`Pressed`
    (if (not (`self.meleeattack`))
      (`PaperFlipbookComponent.SetFlipbook` (`self.Sprite`) "/Game/BlackKnight/Flipbooks/Personaje_Principal/Ataque.Ataque")
      (`/Engine/EditorBlueprintResources/StandardMacros.DoOnce` false :!label _label
        (:`Completed`
          (set `self.meleeattack` true)
          (`KismetSystemLibrary.Delay` 0.2)
          (goto _label :!via `Reset`))))))

(event `Meleeattacking`
  (`/Game/BlackKnight/Blueprints/Components/AttackComponent.MeleeTraceAttack` :`self` (`self.AttackComponent`) :`AttackDuration` 0.1))

(event `self.OnLanded`
  (params (Hit :type "HitResult Structure (by ref)"))
  (set `self.falling` false)
  (set `self.jumping` false))

(event `InputAction|Salto`
  (params (Key :type "Key Structure"))
  (bind _charactermovementcomponent (`self.CharacterMovementComponent`))
  (:`Pressed`
    (bind _canjump_ (`/Game/BlackKnight/Blueprints/Components/CharacterMovementComponent.Jump` _charactermovementcomponent 0.0))
    (if _canjump_
      (set `self.jumping` true)
      (`PaperFlipbookComponent.SetFlipbook` (`self.Sprite`) "/Game/BlackKnight/Flipbooks/Personaje_Principal/Salto.Salto")
      (`KismetSystemLibrary.Delay` 0.1)
      (set `self.jumping` false)
      (set `self.falling` true)))
  (:`Released`
    (`/Game/BlackKnight/Blueprints/Components/CharacterMovementComponent.EndJumping` _charactermovementcomponent)))

(event `InputAxis|MovimientoDerecha`
  (params (AxisValue :type "Float (single-precision)"))
  (bind _returnvalue (`self.GetController`))
  (bind (_ismoving _canturn_) (`/Game/BlackKnight/Blueprints/Components/CharacterMovementComponent.Move` (`self.CharacterMovementComponent`) (`GameplayStatics.GetPlayerPawn` 0) AxisValue))
  (set `self.isMoving` _ismoving)
  (if _canturn_
    (`/Engine/EditorBlueprintResources/StandardMacros.CompareFloat` AxisValue
      (:`>`
        (`Controller.SetControlRotation` _returnvalue (`KismetMathLibrary.MakeRotator` 0.0))
        (`PaperFlipbookComponent.SetFlipbook` (`self.Sprite`) "/Game/BlackKnight/Flipbooks/Personaje_Principal/Run1.Run1" :!label _label_2))
      (:`==`
        (`PaperFlipbookComponent.SetFlipbook` (`self.Sprite`) "/Game/BlackKnight/Flipbooks/Personaje_Principal/Estatico.Estatico"))
      (:`<`
        (`Controller.SetControlRotation` _returnvalue (`KismetMathLibrary.MakeRotator` 0.0 0.0 180.0))
        (goto _label_2)))))

(event `self.ReceiveBeginPlay`
  (bind _returnvalue (`GameplayStatics.GetPlayerController` 0))
  (`PlayerController.SetViewTargetWithBlend` _returnvalue (`ActorComponent.GetOwner` (`self.Camera`)) 0.1 "VTBlend_Linear" 0.0 false)
  (`WidgetBlueprintLibrary.SetInputMode_GameOnly` _returnvalue))

(fn `UserConstructionScript`)