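; Player character for a 2D pixel-art game, with movement, jumping, melee attack and pause menu.
; Input drives the pixel movement component, turns by control yaw, and sets state flags for moving, jumping, falling and attacking.
; Q starts a cooldown-gated attack; a separate MeleeAttackStart event runs the attack component's socket trace.
; Damage feeds the health component, shown on the HUD; zero health spawns a death explosion and opens a paused Game Over screen.
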(event `InputAction|Pausa`
  (params (Key :type "Key Structure"))
  (bind _returnvalue (`GameplayStatics.GetPlayerController` 0))
  ;[1 1 1] PAUSA
  (:`Pressed`
    (bind _returnvalue_2 (`|CreateWidget` "/Game/BlackKnight/Blueprints/menupausa.menupausa_C" _returnvalue))
    (`UserWidget.AddToPlayerScreen` _returnvalue_2 0)
    (`WidgetBlueprintLibrary.SetInputMode_UIOnlyEx` _returnvalue _returnvalue_2)
    (set `PlayerController.bShowMouseCursor` true _returnvalue)
    (`GameplayStatics.SetGamePaused` true)))

(event `self.OnLanded`
  (params (Hit :type "HitResult Structure (by ref)"))
  (set `self.falling` false)
  (set `self.jumping` false))

(event `InputAction|Salto`
  (params (Key :type "Key Structure"))
  (bind _bp_pixelcharactermovementcomponent (`self.BP_PixelCharacterMovementComponent`))
  (:`Pressed`
    (bind _canjump_ (`/Game/Pixel2D/Blueprints/Components/BP_PixelCharacterMovementComponent.Jump` _bp_pixelcharactermovementcomponent 0.0))
    (if _canjump_
      (set `self.jumping` true)
      (`KismetSystemLibrary.Delay` 0.2)
      (set `self.jumping` false)
      (set `self.falling` true)))
  (:`Released`
    (`/Game/Pixel2D/Blueprints/Components/BP_PixelCharacterMovementComponent.EndJumping` _bp_pixelcharactermovementcomponent)))

(event `InputAxis|MovimientoDerecha`
  (params (AxisValue :type "Float (single-precision)"))
  (bind _returnvalue (`self.GetController`))
  (bind (_ismoving _canturn_) (`/Game/Pixel2D/Blueprints/Components/BP_PixelCharacterMovementComponent.Move` (`self.BP_PixelCharacterMovementComponent`) (`GameplayStatics.GetPlayerPawn` 0) AxisValue))
  (set `self.isMoving` _ismoving)
  (if _canturn_
    (`/Engine/EditorBlueprintResources/StandardMacros.CompareFloat` AxisValue
      (:`>`
        (`Controller.SetControlRotation` _returnvalue (`KismetMathLibrary.MakeRotator` 0.0)))
      (:`<`
        (`Controller.SetControlRotation` _returnvalue (`KismetMathLibrary.MakeRotator` 0.0 0.0 180.0))))))

(event `self.ReceiveBeginPlay`
  (bind _returnvalue (`GameplayStatics.GetPlayerController` 0))
  (`PlayerController.SetViewTargetWithBlend` _returnvalue (`ActorComponent.GetOwner` (`self.Camera`)) 0.1 "VTBlend_Linear" 0.0 false)
  (bind _returnvalue_2 (`|CreateWidget` "/Game/BlackKnight/Blueprints/widgets/MainWidget.MainWidget_C" null (`self.BP_HealthComponent`)))
  (`UserWidget.AddToViewport` _returnvalue_2 0)
  (`WidgetBlueprintLibrary.SetInputMode_GameOnly` _returnvalue))

(event `self.BP_HealthComponent.HealthChanged`
  (params (`New Value` :type Integer) (Change :type "/Game/Pixel2D/Blueprints/Enums/E_StatChange Enum" :default "NewEnumerator0") (Instigator :type "Actor Object Reference"))
  (bind _returnvalue (`GameplayStatics.GetPlayerController` 0))
  (if (<= `New Value` 0)
    (`WidgetLayoutLibrary.RemoveAllWidgets`)
    (`/Game/Pixel2D/Blueprints/Components/BP_HealthComponent.DestroyActorOnDeath` (`self.BP_HealthComponent`) self (`self.PixelComponent`) 0.0 (`|MakeArray` "/Game/Pixel2D/Blueprints/Objects/BP_DeathExplode.BP_DeathExplode_C" :!type "Actor Class Reference") null null)
    (bind _returnvalue_2 (`|CreateWidget` "/Game/BlackKnight/Blueprints/GameOver.GameOver_C"))
    (`WidgetBlueprintLibrary.SetInputMode_UIOnlyEx` _returnvalue null)
    (`UserWidget.AddToPlayerScreen` _returnvalue_2 0)
    (set `PlayerController.bShowMouseCursor` true _returnvalue)
    (`GameplayStatics.SetGamePaused` true)))

(event `MeleeAnimationFinished`
  (set `self.meleeattack` false))

(event `Key|Q`
  (params (Key :type "Key Structure"))
  (:`Pressed`
    (if (not (`self.meleeattack`))
      (`/Engine/EditorBlueprintResources/StandardMacros.DoOnce` false :!label _label
        (:`Completed`
          (set `self.meleeattack` true)
          (`KismetSystemLibrary.Delay` (`self.meleeAttackSpeed`))
          (goto _label :!via `Reset`))))))

(event `MeleeAttackStart`
  (`/Game/Pixel2D/Blueprints/Components/BP_AttackComponent.MeleeTraceAttack` (`self.BP_AttackComponent`) "HitSocket" (`self.PixelComponent`) (`self.meleeDamage`) (`self.meleeAttackSpeed`) 0.0 5.0 (struct :`R` 1.0 :`G` 0.010417 :`B` 0.010417 :`A` 1.0) (`self.knockbackForce`) (`self.enemyTag`)))

(event `self.ReceiveAnyDamage`
  (params (Damage :type "Float (single-precision)") (DamageType :type "DamageType Object Reference") (InstigatedBy :type "Controller Object Reference") (DamageCauser :type "Actor Object Reference"))
  (`/Game/Pixel2D/Blueprints/Components/BP_HealthComponent.DecreaseHealth` (`self.BP_HealthComponent`) (`KismetMathLibrary.FTrunc` Damage) (0.0 0.0 0.0) null))

(fn `GetEnemyTagContainer`
  (returns (EnemyTags :type "GameplayTagContainer Structure"))
  (return (`self.enemyTag`)))

(fn `GetGameplayTagContainer`
  (returns (TagContainer :type "GameplayTagContainer Structure"))
  (return (`self.ownedTags`)))

(fn `UserConstructionScript`)